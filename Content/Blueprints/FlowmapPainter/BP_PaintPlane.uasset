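; Flowmap painting surface actor, hidden in game, that paints and erases flow data in the RT_Flowmap render target.
; Construction creates dynamic brush and eraser material instances, and BeginPlay optionally clears the target to black.
; Draw and Erase convert a world location into normalized plane coordinates using the PaintPlane bounds, set position and radius on their material, then draw it to the target.
; Draw also passes velocity to the brush.
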(event `self.ReceiveBeginPlay`
  (if (`self.EraseOnStart`)
    (`KismetRenderingLibrary.ClearRenderTarget2D` "/Game/Blueprints/FlowmapPainter/Resources/RT/RT_Flowmap.RT_Flowmap")))

(event `Draw`
  (params (Position :type "Vector Structure") (Velocity :type "Vector Structure") (`Brush Size` :type "Float (double-precision)"))
  (bind _brush (`self.Brush`))
  (`MaterialInstanceDynamic.SetVectorParameterValue` (`self.Brush`) "Position" (`KismetMathLibrary.Conv_VectorToLinearColor` (+ (/ (`KismetMathLibrary.InverseTransformLocation` (`self.GetTransform`) Position) (/ (* (.x (`.BoxExtent` (`KismetSystemLibrary.GetComponentBounds` (`self.PaintPlane`)))) 2.0) (`SceneComponent.K2_GetComponentScale` (`self.PaintPlane`)))) (0.5 0.5 0.5))))
  (`MaterialInstanceDynamic.SetVectorParameterValue` _brush "Velocity" (`KismetMathLibrary.Conv_VectorToLinearColor` Velocity))
  (`MaterialInstanceDynamic.SetScalarParameterValue` _brush "Radius" `Brush Size`)
  (`KismetRenderingLibrary.DrawMaterialToRenderTarget` "/Game/Blueprints/FlowmapPainter/Resources/RT/RT_Flowmap.RT_Flowmap" (`self.Brush`)))

(event `Erase`
  (params (Location :type "Vector Structure") (radius :type "Float (double-precision)"))
  (`MaterialInstanceDynamic.SetVectorParameterValue` (`self.Eraser`) "Position" (`KismetMathLibrary.Conv_VectorToLinearColor` (+ (/ (`KismetMathLibrary.InverseTransformLocation` (`self.GetTransform`) Location) (/ (* (.x (`.BoxExtent` (`KismetSystemLibrary.GetComponentBounds` (`self.PaintPlane`)))) 2.0) (`SceneComponent.K2_GetComponentScale` (`self.PaintPlane`)))) 0.5)))
  (`MaterialInstanceDynamic.SetScalarParameterValue` (`self.Eraser`) "Radius" radius)
  (`KismetRenderingLibrary.DrawMaterialToRenderTarget` "/Game/Blueprints/FlowmapPainter/Resources/RT/RT_Flowmap.RT_Flowmap" (`self.Eraser`)))

(fn `UserConstructionScript`
  (bind _returnvalue (`KismetMaterialLibrary.CreateDynamicMaterialInstance` "/Game/Blueprints/FlowmapPainter/Resources/RT/M_Brush_PaintFM.M_Brush_PaintFM"))
  (set `self.Brush` _returnvalue)
  (bind _returnvalue_2 (`KismetMaterialLibrary.CreateDynamicMaterialInstance` "/Game/Blueprints/FlowmapPainter/Resources/RT/M_Brush_EraseFM.M_Brush_EraseFM"))
  (set `self.Eraser` _returnvalue_2)
  (`self.SetActorHiddenInGame` true))