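; BP_Stream is a stream actor that bakes a flow-map mask and jump-flood distance field at BeginPlay for a Niagara system.
; An orthographic scene capture renders only the stream plane and occluder mesh, briefly swapped to capture materials.
; JumpFloodComponent2D floods a seed mask texture into ping-pong render targets, shown through a debug material; the gradient pass is never run.
; The construction script sizes plane, capture width and Niagara scale from PlaneScale.
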(event `Send Niagara Textures`
  (`NiagaraComponent.SetVariableTexture` (`self.StreamSystem`) "JF_Tex" null))

(event `self.ReceiveBeginPlay`
  (`|ExecutionSequence`
    (:`then_0`
      (`self.Generate RT_1 (Mask)`))
    (:`then_1`
      (`self.Generate RT 2 (SDF)`))
    (:`then_2`
      (`self.Send Niagara Textures`))))

(event `Generate RT_1 (Mask)`
  ;[0 0 0] Capture river texture (RGBA)
  (`self.SetCaptureAllow`)
  (`self.SetCaptureMaterials` true)
  (`KismetSystemLibrary.DelayUntilNextTick`)
  (`SceneCaptureComponent2D.CaptureScene` (`self.SceneCaptureComponent2D`))
  (`self.SetCaptureMaterials` false))

(event `Generate RT 2 (SDF)`
  (bind _jumpfloodcomponent_2d (`self.JumpFloodComponent_2D`))
  ;[0 0 0] Jumpflood / SDF from texture (2nd RT)
  (`KismetSystemLibrary.DelayUntilNextTick`)
  (set `/Volumetrics/Tools/JumpFlooding/Blueprints/JumpFloodComponent_2D.RT A` (`self.RT_JFA`) _jumpfloodcomponent_2d)
  (set `/Volumetrics/Tools/JumpFlooding/Blueprints/JumpFloodComponent_2D.RT B` (`self.RT_JFA_Buffer`) _jumpfloodcomponent_2d)
  (`self.1) Clear RTs`)
  (`self.2) Jump Flood`))

(event `SetCaptureMaterials`
  (params (On :type Boolean))
  ;[0 0 0] Capture river texture (RGBA)
  (`PrimitiveComponent.SetMaterial` (`self.StreamPlane`) 0 (select `bool` On :`false` "/Game/Blueprints/Stream/M_StreamSurface.M_StreamSurface" :`true` "/Game/Blueprints/Stream/M_CAPTUREMAT_FLOWMAP.M_CAPTUREMAT_FLOWMAP" :!type "MaterialInterface Object Reference"))
  (bind _asstatic_mesh_actor (cast `StaticMeshActor` (`self.OccluderMeshes`)))
  (`PrimitiveComponent.SetMaterial` (`StaticMeshActor.StaticMeshComponent` _asstatic_mesh_actor) 0 (select `bool` On :`false` "/Game/Blueprints/Sample/MeshLandscape/M_MeshLandscape.M_MeshLandscape" :`true` "/Game/Blueprints/Sample/MeshLandscape/M_CaptureMask.M_CaptureMask" :!type "MaterialInterface Object Reference")))

(event `1) Clear RTs`
  (bind _jumpfloodcomponent_2d (`self.JumpFloodComponent_2D`))
  (bind _jumpfloodcomponent_2d_2 (`self.JumpFloodComponent_2D`))
  ;[0 0 0] Jumpflood / SDF from texture (2nd RT)
  ;;[0.4896 0.004675 0] Debug Reset Button
  (`KismetRenderingLibrary.ClearRenderTarget2D` (`/Volumetrics/Tools/JumpFlooding/Blueprints/JumpFloodComponent_2D.RT A` _jumpfloodcomponent_2d))
  (`KismetRenderingLibrary.ClearRenderTarget2D` (`/Volumetrics/Tools/JumpFlooding/Blueprints/JumpFloodComponent_2D.RT B` _jumpfloodcomponent_2d))
  (set `/Volumetrics/Tools/JumpFlooding/Blueprints/JumpFloodComponent_2D.CurrentIndex` 0 _jumpfloodcomponent_2d_2)
  (set `/Volumetrics/Tools/JumpFlooding/Blueprints/JumpFloodComponent_2D.StartIndex` 0 _jumpfloodcomponent_2d_2))

(event `SetCaptureAllow`
  (bind _scenecapturecomponent2d (`self.SceneCaptureComponent2D`))
  ;[0 0 0] Capture river texture (RGBA)
  (`SceneCaptureComponent.ShowOnlyComponent` _scenecapturecomponent2d (`self.StreamPlane`))
  (`SceneCaptureComponent.ShowOnlyActorComponents` _scenecapturecomponent2d (`self.OccluderMeshes`) false))

(event `2) Jump Flood`
  ;[0 0 0] Jumpflood / SDF from texture (2nd RT)
  ;;[1 1 1] How to use the component when specifying a mask texture
  (bind _result_rt (`/Volumetrics/Tools/JumpFlooding/Blueprints/JumpFloodComponent_2D.Jump Flood` (`self.JumpFloodComponent_2D`) (`self.Seed Mode`) (`self.Mask Texture`) (`self.Smoothing Passes`)))
  (`MaterialInstanceDynamic.SetTextureParameterValue` (`self.Debug RT MID`) "RT" _result_rt))

(event `3) Gradient`
  ;[0 0 0] Jumpflood / SDF from texture (2nd RT)
  ;;[1 1 1] Gradient
  (bind _result_rt (`/Volumetrics/Tools/JumpFlooding/Blueprints/JumpFloodComponent_2D.Compute Gradient` (`self.JumpFloodComponent_2D`)))
  (set `self.JumpFloodTexture` _result_rt)
  (`MaterialInstanceDynamic.SetTextureParameterValue` (`self.Debug RT MID`) "RT" _result_rt))

(fn `UserConstructionScript`
  (bind _planescale (`self.PlaneScale`))
  (bind _debug_rt_mid (`self.Debug RT MID`))
  (`|ExecutionSequence`
    (:`then_0`
      (`SceneComponent.SetRelativeScale3D` (`self.StreamPlane`) (`KismetMathLibrary.Conv_DoubleToVector` _planescale))
      (set `SceneCaptureComponent2D.OrthoWidth` (* _planescale 100.0) (`self.SceneCaptureComponent2D`))
      (`NiagaraComponent.SetVariableFloat` (`self.StreamSystem`) "bp_scale" (`self.PlaneScale`)))
    (:`then_1`
      (`/Volumetrics/Tools/BlueprintLibraries/VolumetricsBPLIbrary.Create and Assign MID` (`self.Debug RT MID`) "/Volumetrics/Tools/JumpFlooding/Materials/Debug/M_Debug_DistanceField_Texels.M_Debug_DistanceField_Texels")
      (`MaterialInstanceDynamic.SetScalarParameterValue` _debug_rt_mid "ShowGrid" (`KismetMathLibrary.Conv_BoolToDouble` (`self.Show Grid`)))
      (`MaterialInstanceDynamic.SetScalarParameterValue` _debug_rt_mid "ShowDistance" (`KismetMathLibrary.Conv_BoolToDouble` (`self.Show Distance`)))
      (`MaterialInstanceDynamic.SetScalarParameterValue` _debug_rt_mid "ShowGradient" (`KismetMathLibrary.Conv_BoolToDouble` (`self.Show Gradient`)))
      (`MaterialInstanceDynamic.SetScalarParameterValue` _debug_rt_mid "DistanceDivisor" (`self.Distance Divisor`)))))