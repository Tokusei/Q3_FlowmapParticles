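; Pawn for painting flow onto the first BP_Stream actor found in the level, with key hints printed on screen.
; Each tick it traces under the cursor, moves a brush sphere there, and derives velocity from the hit-point delta scaled by intensity.
; Left mouse draws that velocity into the stream and right mouse erases.
; Wheel resizes the brush, keys adjust intensity, toggle look lock and toggle the flowmap preview.
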(event `self.ReceiveBeginPlay`
  (`KismetSystemLibrary.PrintString` "TAB: Lock view ON/OFF" true true (struct :`R` 1.0 :`G` 0.327889 :`A` 1.0) 44.0)
  (`KismetSystemLibrary.PrintString` "1/2: +/- Intensity" true true (struct :`R` 1.0 :`G` 0.327889 :`A` 1.0) 44.0)
  (`KismetSystemLibrary.PrintString` "3: Show/Hide flowmap" true true (struct :`R` 1.0 :`G` 0.327889 :`A` 1.0) 44.0)
  (set `PlayerController.bShowMouseCursor` false (`GameplayStatics.GetPlayerController` 0))
  (bind _outactors (`GameplayStatics.GetAllActorsOfClass` "/Game/Blueprints/BP_Stream.BP_Stream_C"))
  (set `self.BP_Stream` (`|GetArrayItem` _outactors)))

(event `Key|Three`
  (params (Key :type "Key Structure"))
  (:`Pressed`
    (bind _isa (`/Engine/EditorBlueprintResources/StandardMacros.FlipFlop`)
      (:`A`
        _)
      (:`B`
        _))
    (`/Game/Blueprints/BP_Stream.FM_Preview` (`self.BP_Stream`) _isa)))

(event `InputAxisKey|MouseWheelAxis`
  (params (AxisValue :type "Float (single-precision)"))
  (set `self.Brush Size` (`KismetMathLibrary.FClamp` (+ (`self.Brush Size`) (* AxisValue 0.003)) 0.0 10.0))
  (`SceneComponent.SetWorldScale3D` (`self.Sphere`) (`KismetMathLibrary.Conv_DoubleToVector` (* (`self.Brush Size`) 15.0))))

(event `Key|Tab`
  (params (Key :type "Key Structure"))
  (:`Pressed`
    (bind _isa (`/Engine/EditorBlueprintResources/StandardMacros.FlipFlop`)
      (:`A`
        _)
      (:`B`
        _))
    (`Controller.SetIgnoreLookInput` (`self.GetController`) _isa)
    (`KismetSystemLibrary.PrintString` (`KismetStringLibrary.Concat_StrStr` "View lock: " (`KismetStringLibrary.Conv_BoolToString` _isa)))))

(event `Key|One`
  (params (Key :type "Key Structure"))
  (:`Pressed`
    (bind _output_get (set `self.Intensity` (+ (`self.Intensity`) 0.05)))
    (`KismetSystemLibrary.PrintString` (`KismetStringLibrary.Conv_DoubleToString` _output_get))))

(event `Key|LeftMouseButton`
  (params (Key :type "Key Structure"))
  (:`Pressed`
    (set `self.LeftMouseDown?` true))
  (:`Released`
    (set `self.LeftMouseDown?` false)))

(event `Key|RightMouseButton`
  (params (Key :type "Key Structure"))
  (:`Pressed`
    (set `self.RightMouseButton` true))
  (:`Released`
    (set `self.RightMouseButton` false)))

(event `Key|Two`
  (params (Key :type "Key Structure"))
  (:`Pressed`
    (bind _output_get (set `self.Intensity` (+ (`self.Intensity`) -0.05)))
    (`KismetSystemLibrary.PrintString` (`KismetStringLibrary.Conv_DoubleToString` _output_get))))

(event `self.ReceiveTick`
  (params (DeltaSeconds :type "Float (single-precision)"))
  (`self.Trace Under Mouse`)
  (`self.Update Sphere Loc`)
  (`|ExecutionSequence`
    (:`then_0`
      (if (`self.LeftMouseDown?`)
        (bind _output_get (set `self.Velocity` (* (`self.Mouse Velocity`) (`self.Intensity`))))
        (`/Game/Blueprints/BP_Stream.Draw` (`self.BP_Stream`) (`self.Position`) _output_get (`self.Brush Size`))))
    (:`then_1`
      (if (`self.RightMouseButton`)
        (`/Game/Blueprints/BP_Stream.Erase` (`self.BP_Stream`) (`self.Position`) (`self.Brush Size`))))))

(fn `Trace Under Mouse`
  (bind (_hitresult _returnvalue) (`PlayerController.GetHitResultUnderCursorByChannel` (`GameplayStatics.GetPlayerController` 0) "TraceTypeQuery1" true))
  (if _returnvalue
    (set `self.Mouse Velocity` (- (`.Location` (`GameplayStatics.BreakHitResult` _hitresult)) (`self.Position`)))
    (set `self.Position` (`.Location` (`GameplayStatics.BreakHitResult` _hitresult)))
    (return)))

(fn `Update Sphere Loc`
  (`SceneComponent.K2_SetWorldLocation` (`self.Sphere`) (`self.Position`) false false))

(fn `UserConstructionScript`)